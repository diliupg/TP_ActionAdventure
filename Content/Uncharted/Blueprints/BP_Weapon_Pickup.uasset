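; BP_Weapon_Pickup is a weapon pickup actor that the player collects by pressing E.
; TriggerVolume overlaps with a ThirdPersonCharacter toggle a text prompt and the CanPickUpWeapon flag.
; Pressing E while allowed marks it picked up, plays a 2D sound and destroys the actor, without granting a weapon itself.
; Tick orients the text from the player controller's rotation plus a 180-degree flip.
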(event `self.TriggerVolume.OnComponentBeginOverlap`
  (params (OverlappedComponent :type "PrimitiveComponent Object Reference") (OtherActor :type "Actor Object Reference") (OtherComp :type "PrimitiveComponent Object Reference") (OtherBodyIndex :type Integer) (bFromSweep :type Boolean) (SweepResult :type "HitResult Structure (by ref)"))
  ;[0.6278 0.8888 1] Show and Hide PickUp Weapon Message
  (cast `/Game/ThirdPersonBP/Blueprints/ThirdPersonCharacter` OtherActor)
  (if (not (`self.HasWeaponBeenPickedUp`))
    (`SceneComponent.SetVisibility` (`self.TextRender`) true false)
    (set `self.CanPickUpWeapon` true)))

(event `self.TriggerVolume.OnComponentEndOverlap`
  (params (OverlappedComponent :type "PrimitiveComponent Object Reference") (OtherActor :type "Actor Object Reference") (OtherComp :type "PrimitiveComponent Object Reference") (OtherBodyIndex :type Integer))
  ;[0.6278 0.8888 1] Show and Hide PickUp Weapon Message
  (cast `/Game/ThirdPersonBP/Blueprints/ThirdPersonCharacter` OtherActor)
  (`SceneComponent.SetVisibility` (`self.TextRender`) false false)
  (set `self.CanPickUpWeapon` false))

(event `Key|E`
  (params (Key :type "Key Structure"))
  ;[1 1 1] Pick up Weapon
  (:`Pressed`
    (if (`self.CanPickUpWeapon`)
      (`SceneComponent.SetVisibility` (`self.TextRender`) true false)
      (set `self.HasWeaponBeenPickedUp` true)
      (`GameplayStatics.PlaySound2D` "/Game/Uncharted/Sound/EFX/WeaponPick-Up.WeaponPick-Up" 1.0 1.0 0.0 null null)
      (`self.K2_DestroyActor`))))

(event `self.ReceiveTick`
  (params (DeltaSeconds :type "Float (single-precision)"))
  (bind _textrender (`self.TextRender`))
  ;[1 1 1] Text Rotation
  (`SceneComponent.K2_SetWorldRotation` _textrender (.rotation (`self.GetTransform` (`GameplayStatics.GetPlayerController` 0))) false false)
  (`SceneComponent.K2_AddLocalRotation` _textrender (struct :`Yaw` 180.0) false false))

(fn `UserConstructionScript`)