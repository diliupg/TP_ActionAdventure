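; BP_TreasurePickup is a treasure pickup actor that the player collects by pressing E while inside its trigger box.
; Overlapping the TriggerBox shows the Icon prompt and enables pickup until treasure is taken; only the end overlap, which reverses this, checks for ThirdPersonCharacter.
; Pressing E while enabled marks the treasure as picked up, plays a 2D found-treasure sound and destroys the actor.
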(event `self.TriggerBox.OnComponentBeginOverlap`
  (params (OverlappedComponent :type "PrimitiveComponent Object Reference") (OtherActor :type "Actor Object Reference") (OtherComp :type "PrimitiveComponent Object Reference") (OtherBodyIndex :type Integer) (bFromSweep :type Boolean) (SweepResult :type "HitResult Structure (by ref)"))
  ;[0.6278 0.8888 1] Show and Hide PickUp Treasure Message
  (if (not (`self.HasTreasureBeenPickedUp`))
    (`SceneComponent.SetVisibility` (`self.Icon`) true false)
    (set `self.CanPickUpTreasure` true)))

(event `self.TriggerBox.OnComponentEndOverlap`
  (params (OverlappedComponent :type "PrimitiveComponent Object Reference") (OtherActor :type "Actor Object Reference") (OtherComp :type "PrimitiveComponent Object Reference") (OtherBodyIndex :type Integer))
  ;[0.6278 0.8888 1] Show and Hide PickUp Treasure Message
  (cast `/Game/ThirdPersonBP/Blueprints/ThirdPersonCharacter` OtherActor)
  (`SceneComponent.SetVisibility` (`self.Icon`) false false)
  (set `self.CanPickUpTreasure` false))

(event `Key|E`
  (params (Key :type "Key Structure"))
  ;[1 1 1] Pick up Treasure
  (:`Pressed`
    (if (`self.CanPickUpTreasure`)
      (`SceneComponent.SetVisibility` (`self.Icon`) true false)
      (set `self.HasTreasureBeenPickedUp` true)
      (`GameplayStatics.PlaySound2D` "/Game/Uncharted/Sound/EFX/FoundTreasureSoundEffect.FoundTreasureSoundEffect" 1.0 1.0 0.0 null null)
      (`self.K2_DestroyActor`))))

(fn `UserConstructionScript`)